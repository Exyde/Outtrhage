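; BP_Bloodlet is a projectile actor, apparently a blood droplet, that stops where it first touches something.
; Launch sets the ProjectileMovement velocity from a given speed and direction.
; When Sphere1 overlaps another actor, it prints that actor's name and zeroes velocity and gravity scale, leaving the projectile suspended in place without destroying it.
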(event OnComponentBeginOverlap(Sphere1)
  (params (OverlappedComponent :type Primitive%20Component%20Object%20Reference) (OtherActor :type Actor%20Object%20Reference) (OtherComp :type Primitive%20Component%20Object%20Reference) (OtherBodyIndex :type Integer) (bFromSweep :type Boolean) (SweepResult :type Hit%20Result%20Structure%20%28by%20ref%29))
  (bind _projectilemovement (Variables|Default|GetProjectileMovement))
  (if (!= OtherActor self)
    (Development|PrintString (Utilities|GetDisplayName OtherActor))
    (Variables|/Script/Engine.MovementComponent|SetVelocity _projectilemovement "0, 0, 0")
    (Variables|/Script/Engine.ProjectileMovementComponent|SetProjectileGravityScale _projectilemovement 0.0)))

(fn ConstructionScript)

(fn Launch
  (params (Speed :type Float%20%28double-precision%29) (Direction :type Vector))
  (Variables|/Script/Engine.MovementComponent|SetVelocity (Variables|Default|GetProjectileMovement) (* Speed Direction)))