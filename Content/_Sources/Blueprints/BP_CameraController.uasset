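; BP_CameraController is a camera actor that becomes the player's view target and follows the BP_Riel character.
; On BeginPlay it sets the FOV, stores the player as its target, and can lock pitch to the true isometric arcsin(1/√3) angle at a configurable yaw.
; Each tick it repositions its root at the target plus an offset, pulled back along the camera's forward vector by a set distance.
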(event EventBeginPlay
  (Development|PrintString "Hello")
  (Utilities|FlowControl|Sequence
    (:then_0
      (Variables|Default|SetIsometric%20Arc%20Sin%20Angle (|(asind((1/(sqrt(3))))))))
    (:then_1
      (if (Variables|Default|GetForceIsoLockRotation)
        (Transformation|SetRelativeRotation (Variables|Default|GetCamera) (Math|Rotator|MakeRotator 0.0 (* (Variables|Default|GetIsometric%20Arc%20Sin%20Angle) -1.0) (Variables|Default|GetCamera%20Rotation)) false false)))
    (:then_2
      (Transformation|SetWorldLocation (Variables|Default|GetDefaultSceneRoot) (+ (* (Math|Vector|GetForwardVector (Variables|Default|GetCamera)) (* (Variables|Default|GetDistance) -1.0)) (Variables|Default|GetCamera%20Offset)) false false))
    (:then_3
      (Camera|SetFieldOfView (Variables|Default|GetCamera) (Variables|Default|GetFOV)))
    (:then_4
      (Game|Player|SetViewTargetwithBlend (Game|GetPlayerController 0) self 0.0 "VTBlend_Linear" 0.0 false))
    (:then_5
      (bind _asbp_riel (Utilities|Casting|CastToBP_Riel (Game|GetPlayerCharacter 0)))
      (bind _output_get (Variables|Default|SetPlayer _asbp_riel))
      (Variables|Default|SetTarget _output_get))))

(event EventTick
  (params (DeltaSeconds :type Float%20%28single-precision%29))
  (Transformation|SetWorldLocation (Variables|Default|GetDefaultSceneRoot) (+ (* (Math|Vector|GetForwardVector (Variables|Default|GetCamera)) (* (Variables|Default|GetDistance) -1.0)) (Variables|Default|GetCamera%20Offset) (Transformation|GetActorLocation (Variables|Default|GetTarget))) false false))

(fn ConstructionScript)